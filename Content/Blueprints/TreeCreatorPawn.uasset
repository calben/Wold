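; Pawn that spawns procedurally generated trees at preset spawn locations through its SpawnTree event.
; Each call advances a wrapping index into SpawnLocations, ignoring the TreeTransform input, and spawns a parameterised tree generator there.
; One seed drives trunk, branches and leaves, alongside irregularity, colour and leaf amount inputs.
; OccupiedLocations tracks the tree in each slot, so the previous occupant is destroyed and replaced.
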(event Custom|SpawnTree
  (params (TreeTransform :type Transform) (RandomSeed :type Integer) (TrunkIrregularity :type Float%20%28single-precision%29) (LeafColor :type Linear%20Color%20Structure) (BarkColor :type Linear%20Color%20Structure) (LeavesAmount :type Integer))
  (bind _spawnlocations (Variables|Default|GetSpawnLocations))
  (if (< (Variables|Default|GetCurrentSpawnIndex) (Utilities|Array|Length _spawnlocations))
    (Math|Integer|IncrementInt (Variables|Default|GetCurrentSpawnIndex)
      (:%20%20
        _))
    (else
      (Variables|Default|SetCurrentSpawnIndex 0)))
  (bind _returnvalue (Game|SpawnActorfromClass "/Game/Blueprints/SpawnParameterisedTreeGeneratpr_BP.SpawnParameterisedTreeGeneratpr_BP_C" (Utilities|Array|Get(acopy) _spawnlocations (Variables|Default|GetCurrentSpawnIndex)) "AdjustIfPossibleButAlwaysSpawn" 0 RandomSeed RandomSeed RandomSeed RandomSeed TrunkIrregularity LeafColor BarkColor LeavesAmount 0))
  (if (!= (Utilities|Array|Get(acopy) (Variables|Default|GetOccupiedLocations) (Variables|Default|GetCurrentSpawnIndex)) 0)
    (Actor|DestroyActor (Utilities|Array|Get(acopy) (Variables|Default|GetOccupiedLocations) (Variables|Default|GetCurrentSpawnIndex))))
  (Utilities|Array|SetArrayElem (Variables|Default|GetOccupiedLocations) (Variables|Default|GetCurrentSpawnIndex) _returnvalue))

(event EventBeginPlay)

(event Collision|EventActorBeginOverlap
  (params (OtherActor :type Actor%20Object%20Reference)))

(event EventTick
  (params (DeltaSeconds :type Float%20%28single-precision%29)))

(fn ConstructionScript)